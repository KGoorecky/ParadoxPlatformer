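; BP_Clock is a clock Blueprint that continuously bobs and rocks its PivotPoint component.
; On BeginPlay, two independent timelines start: Float lerps the relative location up and down, and Rotate lerps the relative rotation side to side.
; Each timeline's Finished output drives a FlipFlop that alternates Reverse and Play, creating an endless ping-pong motion without Tick.
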(event EventBeginPlay
  (Utilities|FlowControl|Sequence
    (:then_0
      (bind _floating (Timeline|Float Play)
        (:Update
          (Transformation|SetRelativeLocation (Variables|Default|GetPivotPoint) (Math|Vector|Lerp(Vector) "0.000000,0.000000,-50.000000" "0.000000,0.000000,50.000000" _floating) false false))
        (:Finished
          (Utilities|FlowControl|FlipFlop
            (:A
              (Timeline|Float Reverse))
            (:B
              (Timeline|Float Play))))))
    (:then_1
      (bind _rotating (Timeline|Rotate Play)
        (:Update
          (Transformation|SetRelativeRotation (Variables|Default|GetPivotPoint) (Math|Rotator|Lerp(Rotator) "0.000000,-15.000000,0.000000" "0.000000,15.000000,0.000000" _rotating) false false))
        (:Finished
          (Utilities|FlowControl|FlipFlop
            (:A
              (Timeline|Rotate Reverse))
            (:B
              (Timeline|Rotate Play))))))))

(fn ConstructionScript)