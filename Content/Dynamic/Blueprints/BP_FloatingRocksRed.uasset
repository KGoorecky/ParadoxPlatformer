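; Decorative floating rock cluster that animates a main rock and four small rocks from BeginPlay.
; Looping timelines spin the main rock and counter-spin the small rocks at staggered angle offsets.
; Other timelines bob the main rock and two scene components vertically, the latter in opposite phase, using FlipFlops on finish to switch direction.
; An additional rotation timeline for the first scene component is unconnected and never runs.
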(event EventBeginPlay
  (Utilities|FlowControl|Sequence
    (:then_0
      ;[0 0 0 0.5] MainRockSpin
      (bind _spinning (Timeline|MainRockSpin Play)
        (:Update
          (Transformation|SetRelativeRotation (Variables|Default|GetMainRock) (Math|Rotator|Lerp(Rotator) "0.000000,0.000000,0.000000" "0.000000,360.000000,0.000000" _spinning) false false))
        (:Finished
          (if true
            (Timeline|MainRockSpin PlayFromStart)))))
    (:then_1
      ;[0 0 0 0.5] MainRockFloat
      (bind _floating (Timeline|MainRockFloat Play)
        (:Update
          (Transformation|SetRelativeLocation (Variables|Default|GetMainRock) (Math|Vector|Lerp(Vector) "0.000000,0.000000,-30.000000" "0.000000,0.000000,30.000000" _floating) false false))
        (:Finished
          (Utilities|FlowControl|FlipFlop
            (:A
              (Timeline|MainRockFloat Reverse))
            (:B
              (Timeline|MainRockFloat Play))))))
    (:then_3
      ;[0 0 0 0.5] MiniRockSpin
      (bind _spinning_2 (Timeline|MniRockSpin Play)
        (:Update
          (Transformation|SetRelativeRotation (Variables|Default|Getsmall-rock1-1) (Math|Rotator|Lerp(Rotator) "0.000000,360.000000,0.000000" "0, 0, 0" _spinning_2) false false)
          (Transformation|SetRelativeRotation (Variables|Default|Getsmall-rock2-1) (Math|Rotator|Lerp(Rotator) "0.000000,330.000000,0.000000" "0.000000,-30.000000,0.000000" _spinning_2) false false)
          (Transformation|SetRelativeRotation (Variables|Default|Getsmall-rock1-2) (Math|Rotator|Lerp(Rotator) "0.000000,300.000000,0.000000" "0.000000,-60.000000,0.000000" _spinning_2) false false)
          (Transformation|SetRelativeRotation (Variables|Default|Getsmall-rock2-2) (Math|Rotator|Lerp(Rotator) "0.000000,270.000000,0.000000" "0.000000,-90.000000,0.000000" _spinning_2) false false))
        (:Finished
          (if true
            (Timeline|MniRockSpin PlayFromStart)))))
    (:then_4
      ;[0 0 0 0.5] MiniRockFloat1
      (bind _spinning_3 (Timeline|MiniRockFloat1 Play)
        (:Update
          (Transformation|SetRelativeLocation (Variables|Default|GetScene1) (Math|Vector|Lerp(Vector) "0.000000,0.000000,-15.000000" "0.000000,0.000000,15.000000" _spinning_3) false false))
        (:Finished
          (Utilities|FlowControl|FlipFlop
            (:A
              (Timeline|MiniRockFloat1 Play))
            (:B
              (Timeline|MiniRockFloat1 Reverse))))))
    (:then_5
      ;[0 0 0 0.5] MiniRockFloat2
      (bind _spinning_4 (Timeline|MiniRockFloat2 Play)
        (:Update
          (Transformation|SetRelativeLocation (Variables|Default|GetScene2) (Math|Vector|Lerp(Vector) "0.000000,0.000000,15.000000" "0.000000,0.000000,-15.000000" _spinning_4) false false))
        (:Finished
          (Utilities|FlowControl|FlipFlop
            (:A
              (Timeline|MiniRockFloat2 Play))
            (:B
              (Timeline|MiniRockFloat2 Reverse))))))))

(fn ConstructionScript)