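; Actor component that gives its TimeActor a time-rewind ability.
; Each tick it records transform and velocity into rolling 120-sample arrays, dropping the oldest when full.
; While IsTimeReversing is true, it instead pops the newest samples, applying the transform with a swept teleport.
; The popped velocity is then passed to SetActorRelativeLocation rather than restored as velocity, with no empty-array check.
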(event EventBeginPlay)

(event EventTick
  (params (DeltaSeconds :type Float%20%28single-precision%29))
  (CallFunction|ActorTimeReversing))

(fn ActorTimeReversing
  (if (Variables|Default|GetisTimeReversing)
    (CallFunction|ActorLastStatusReversing)
    (else
      (CallFunction|ActorStatusTimeSaving))))

(fn ActorLastStatusReversing
  (bind _timeactor (Variables|Default|GettimeActor))
  (bind _timepointvelocity (Variables|Default|GettimePointVelocity))
  (bind _timepointtransformation (Variables|Default|GettimePointTransformation))
  (bind _returnvalue (Utilities|Array|LastIndex _timepointvelocity))
  (bind _returnvalue_2 (Utilities|Array|LastIndex _timepointtransformation))
  (bind _output_get (Variables|Default|SetreversedTransformation (Utilities|Array|Get(acopy) _timepointtransformation _returnvalue_2)))
  (Transformation|SetActorTransform _timeactor _output_get true true)
  (Utilities|Array|RemoveIndex _timepointtransformation _returnvalue_2)
  (bind _output_get_2 (Variables|Default|SetreversedVelocity (Utilities|Array|Get(acopy) _timepointvelocity _returnvalue)))
  (Transformation|SetActorRelativeLocation _timeactor _output_get_2)
  (Utilities|Array|RemoveIndex _timepointvelocity _returnvalue))

(fn ActorStatusTimeSaving
  (bind _timeactor (Variables|Default|GettimeActor))
  (if (< (Utilities|Array|Length (Variables|Default|GettimePointTransformation)) 120) :!label _label
    (Utilities|Array|Add (Variables|Default|GettimePointTransformation) (Transformation|GetActorTransform _timeactor))
    (Utilities|Array|Add (Variables|Default|GettimePointVelocity) (Transformation|GetVelocity _timeactor))
    (else
      (Utilities|Array|RemoveIndex (Variables|Default|GettimePointTransformation))
      (Utilities|Array|RemoveIndex (Variables|Default|GettimePointVelocity))
      (goto _label))))